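; MathOperations is a Blueprint function library that provides a single math helper, Toward.
; Toward steps a float toward a target float by a given amount and clamps the result so that it does not overshoot.
; It subtracts when above the target, adds when below, and returns the target when the two are equal.
; A WasLower flag records the direction, but only the new value is returned.
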(fn Toward
  (params (InFloat :type Float%20%28single-precision%29) (InFloat2 :type Float%20%28single-precision%29) (Value :type Float%20%28single-precision%29))
  (if (> InFloat InFloat2)
    (LocalVariables|SetWasLower false)
    (bind _output_get (LocalVariables|SetNewValue (- InFloat Value)))
    (if (> InFloat2 _output_get)
      (LocalVariables|SetNewValue InFloat2))
    (elif (> InFloat2 InFloat)
      (LocalVariables|SetWasLower true)
      (bind _output_get_2 (LocalVariables|SetNewValue (+ InFloat Value)))
      (if (> _output_get_2 InFloat2)
        (LocalVariables|SetNewValue InFloat2))
      (else
        (LocalVariables|SetNewValue InFloat2))))
  (return (LocalVariables|GetNewValue)))